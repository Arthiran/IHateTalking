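; BP_HelperBox is a trigger actor that shows a one-time helper hint when a BP_Tire enters it.
; On overlap begin, it reveals the HelperText widget in the GameMenu of player 0's BP_PC and sets that controller's ShownHelperText flag so the hint does not appear again.
; When the tire leaves, it hides the text.
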(event `self.ReceiveActorBeginOverlap`
  (params (OtherActor :type "Actor Object Reference"))
  (cast `/Game/Blueprints/Game/BP_Tire` OtherActor)
  (bind _asbp_pc (cast `/Game/Blueprints/Game/BP_PC` (`GameplayStatics.GetPlayerController` 0)))
  (if (not (`/Game/Blueprints/Game/BP_PC.ShownHelperText` _asbp_pc))
    (`Widget.SetVisibility` (`/Game/Blueprints/Game/WBP_GameMenu.HelperText` (`/Game/Blueprints/Game/BP_PC.GameMenu` _asbp_pc)) "Visible")
    (set `/Game/Blueprints/Game/BP_PC.ShownHelperText` true _asbp_pc)))

(event `self.ReceiveActorEndOverlap`
  (params (OtherActor :type "Actor Object Reference"))
  (cast `/Game/Blueprints/Game/BP_Tire` OtherActor)
  (bind _asbp_pc (cast `/Game/Blueprints/Game/BP_PC` (`GameplayStatics.GetPlayerController` 0)))
  (`Widget.SetVisibility` (`/Game/Blueprints/Game/WBP_GameMenu.HelperText` (`/Game/Blueprints/Game/BP_PC.GameMenu` _asbp_pc)) "Hidden"))

(fn `UserConstructionScript`)