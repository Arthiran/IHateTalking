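; BP_Tire is the rolling tire the player controls, able to change direction and jump until it reaches a victory box.
; Tick applies roll torque while angular damping is zero; turning briefly spikes damping as a brake before a timer clears it.
; Touching BP_VictoryBox swaps in the king mesh, locks controls and saves; leaving it shows the end menu after a delay.
; It also saves physics state on EndPlay and pauses through time dilation.
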(event `self.ReceiveBeginPlay`
  (`GameplayStatics.PlaySound2D` "/Game/SoundFX/SFX_CityAmbience.SFX_CityAmbience" 1.0 1.0 0.0 null null)
  (`self.BecomeKing`))

(event `self.ReceiveTick`
  (params (DeltaSeconds :type "Float (single-precision)"))
  (if (`self.CanExecute`)
    (`self.MoveRight` (`self.CurrentDirection`))))

(event `Key|R`
  (params (Key :type "Key Structure"))
  (:`Pressed`
    (`GameplayStatics.OpenLevel` "MainMap")))

(event `self.TireCol.OnComponentBeginOverlap`
  (params (OverlappedComponent :type "PrimitiveComponent Object Reference") (OtherActor :type "Actor Object Reference") (OtherComp :type "PrimitiveComponent Object Reference") (OtherBodyIndex :type Integer) (bFromSweep :type Boolean) (SweepResult :type "HitResult Structure (by ref)"))
  (if (== (`GameplayStatics.GetObjectClass` OtherActor) "/Game/Blueprints/Game/BP_VictoryBox.BP_VictoryBox_C")
    (set `self.IsKing` true)
    (set `self.CurrentDirection` -1.0)
    (bind _asbp_pc (cast `/Game/Blueprints/Game/BP_PC` (`GameplayStatics.GetPlayerController` 0)))
    (set `/Game/Blueprints/Game/BP_PC.StopControls` true _asbp_pc)
    (`self.BecomeKing`)
    (`self.SaveGame`)))

(event `self.TireCol.OnComponentEndOverlap`
  (params (OverlappedComponent :type "PrimitiveComponent Object Reference") (OtherActor :type "Actor Object Reference") (OtherComp :type "PrimitiveComponent Object Reference") (OtherBodyIndex :type Integer))
  (bind _returnvalue (`GameplayStatics.GetPlayerController` 0))
  (if (== (`GameplayStatics.GetObjectClass` OtherActor) "/Game/Blueprints/Game/BP_VictoryBox.BP_VictoryBox_C")
    (`KismetSystemLibrary.Delay` 3.5)
    (bind _asbp_pc (cast `/Game/Blueprints/Game/BP_PC` _returnvalue))
    (bind _gamemenu (`/Game/Blueprints/Game/BP_PC.GameMenu` _asbp_pc))
    (`Widget.SetVisibility` (`/Game/Blueprints/Game/WBP_GameMenu.EndMenu` _gamemenu) "Visible")
    (set `self.JustFinished` true)
    (set `PlayerController.bShowMouseCursor` true _returnvalue)
    (`WidgetBlueprintLibrary.SetInputMode_UIOnlyEx` _returnvalue _gamemenu)))

(event `self.ReceiveEndPlay`
  (params (EndPlayReason :type "EEndPlayReason Enum" :default "Destroyed"))
  (`self.SaveGame`))

(event `self.ReceiveHit`
  (params (MyComp :type "PrimitiveComponent Object Reference") (Other :type "Actor Object Reference") (OtherComp :type "PrimitiveComponent Object Reference") (bSelfMoved :type Boolean) (HitLocation :type "Vector Structure") (HitNormal :type "Vector Structure") (NormalImpulse :type "Vector Structure") (Hit :type "HitResult Structure (by ref)"))
  (set `self.CanJump` true))

(fn `BecomeKing`
  (if (`self.IsKing`)
    (`StaticMeshComponent.SetStaticMesh` (`self.Tire`) "/Game/Models/Tire/KingTire.KingTire")))

(fn `ChangeDirection`
  (params (Direction :type "Float (double-precision)"))
  (if (`self.CanExecute`)
    (`GameplayStatics.PlaySound2D` "/Game/SoundFX/SFX_TireScreech.SFX_TireScreech" 1.0 1.0 0.0 null null)
    (set `self.currentDirection` Direction)
    (`PrimitiveComponent.SetAngularDamping` (`self.TireCol`) 13.0)
    (`KismetSystemLibrary.K2_SetTimer` self "ResetAngularSpeed" 0.4)))

(fn `Jump`
  (if (and (`self.CanJump`) (`self.CanExecute`))
    (`GameplayStatics.PlaySound2D` "/Game/SoundFX/SFX_Jump.SFX_Jump" 1.0 1.0 0.0 null null)
    (`PrimitiveComponent.AddImpulse` (`self.TireCol`) (`KismetMathLibrary.MakeVector` 0.0 0.0 (`self.JumpImpulse`)) "None" false)
    (set `self.CanJump` false) ; Disallow jumping
  ))

(fn `MoveRight`
  (params (Direction :type "Float (double-precision)"))
  (bind _tirecol (`self.TireCol`))
  (if (== (`PrimitiveComponent.GetAngularDamping` _tirecol) 0.0)
    (`PrimitiveComponent.AddTorqueInRadians` _tirecol (`KismetMathLibrary.MakeVector` (* (`self.RollTorque`) Direction -1.0)) "None" false)))

(fn `PauseGame`
  (`GameplayStatics.SetGlobalTimeDilation` 0.0)
  (set `self.CanExecute` false))

(fn `ResetAngularSpeed`
  (`PrimitiveComponent.SetAngularDamping` (`self.TireCol`) 0.0))

(fn `SaveGame`
  (returns (Success :type Boolean))
  (bind _tirecol (`self.TireCol`))
  (bind _returnvalue (`GameplayStatics.CreateSaveGameObject` "/Game/Blueprints/Game/BP_PlayerInfo.BP_PlayerInfo_C"))
  (bind _returnvalue_2 (`PrimitiveComponent.GetPhysicsLinearVelocity` _tirecol "None"))
  (set `/Game/Blueprints/Game/BP_PlayerInfo.PlayerInfo` (make `/Game/Blueprints/Game/Struct_PlayerInfo` (`self.K2_GetActorLocation`) (`self.CurrentDirection`) _returnvalue_2 (`PrimitiveComponent.GetPhysicsAngularVelocityInRadians` _tirecol "None") (`self.IsKing`) (`self.JustFinished`)) _returnvalue)
  (bind _returnvalue_3 (`GameplayStatics.SaveGameToSlot` _returnvalue (`KismetSystemLibrary.GetPlatformUserName`)))
  (return _returnvalue_3))

(fn `UnPauseGame`
  (if (not (`self.JustFinished`))
    (`GameplayStatics.SetGlobalTimeDilation` 1.0)
    (set `self.CanExecute` true)
    (else
      (`GameplayStatics.OpenLevel` "MainMap"))))

(fn `UserConstructionScript`)