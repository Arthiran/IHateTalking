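; BP_MovingRoad is a road piece that shuttles back and forth along a single axis, bouncing off what it hits.
; Each tick it sets the physics linear velocity of ParentCollider to Incrementor, on Z when MoveZ is true and on Y otherwise.
; A hit flips the sign of Incrementor to reverse travel, except when the other actor's class is BP_Tire.
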(event `self.ReceiveTick`
  (params (DeltaSeconds :type "Float (single-precision)"))
  (bind _incrementor (`self.Incrementor`))
  (bind _parentcollider (`self.ParentCollider`))
  (if (`self.MoveZ`)
    (`PrimitiveComponent.SetPhysicsLinearVelocity` _parentcollider (`KismetMathLibrary.MakeVector` 0.0 0.0 _incrementor) false "None")
    (else
      (`PrimitiveComponent.SetPhysicsLinearVelocity` _parentcollider (`KismetMathLibrary.MakeVector` 0.0 _incrementor) false "None"))))

(event `self.ReceiveHit`
  (params (MyComp :type "PrimitiveComponent Object Reference") (Other :type "Actor Object Reference") (OtherComp :type "PrimitiveComponent Object Reference") (bSelfMoved :type Boolean) (HitLocation :type "Vector Structure") (HitNormal :type "Vector Structure") (NormalImpulse :type "Vector Structure") (Hit :type "HitResult Structure (by ref)"))
  (if (not (== (`GameplayStatics.GetObjectClass` Other) "/Game/Blueprints/Game/BP_Tire.BP_Tire_C"))
    (set `self.Incrementor` (* (`self.Incrementor`) -1.0))))

(fn `UserConstructionScript`)